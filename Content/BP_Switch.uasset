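; BP_Switch is a light switch that turns a referenced spot light on and off.
; Each call to its Interacte event flips the IsLightOn flag and sets the light's SpotLightComponent intensity to either a fixed brightness or zero.
; It prints a French on/off debug message with each toggle and has no active BeginPlay, overlap, Tick or construction logic.
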(event EventBeginPlay)

(event Collision|EventActorBeginOverlap
  (params (OtherActor :type Actor%20Object%20Reference)))

(event EventTick
  (params (DeltaSeconds :type Float%20%28single-precision%29)))

(event EventInteracte
  (bind _light (Variables|Default|GetLight))
  (bind _spotlightcomponent (Variables|/Script/Engine.SpotLight|GetSpotLightComponent _light))
  (if (not (Variables|Default|GetIsLightOn))
    (Variables|Default|SetIsLightOn true)
    (Development|PrintString "allume")
    (Rendering|Components|Light|SetIntensity _spotlightcomponent 8.0)
    (else
      (Variables|Default|SetIsLightOn false)
      (Development|PrintString "allume pas")
      (Rendering|Components|Light|SetIntensity _spotlightcomponent 0.0))))

(fn ConstructionScript)